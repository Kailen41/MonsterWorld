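; BP_Red is the top-down flipbook character Red, moved through Enhanced Input.
; BeginPlay adds the IMC_TopDown mapping context, and IA_Move drives world X/Y movement while storing the input as Directionality.
; FUpdateAnimation picks a four-way walk flipbook from that vector while moving, or the matching idle on release, with horizontal input taking priority over vertical.
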(event `self.ReceiveBeginPlay`
  ;[0 0 1] BeginPlay - Enhanced Input Enabled
  (bind _asplayer_controller (cast `PlayerController` (`self.GetController`)))
  (`/Engine/EditorBlueprintResources/StandardMacros.IsValid` _asplayer_controller
    (:`Is Valid`
      (`EnhancedInputSubsystemInterface.AddMappingContext` (pcsubsystem `EnhancedInputLocalPlayerSubsystem` _asplayer_controller) "/Game/_Main/Input/IMC_TopDown.IMC_TopDown" 0 (struct)))))

(event `EnhancedInput|/Game/_Main/Input/InputActions/IA_Move`
  (params (ActionValue :type "Vector2D Structure") (ElapsedSeconds :type "Float (double-precision)") (TriggeredSeconds :type "Float (double-precision)") (InputAction :type "InputAction Object Reference" :default "/Game/_Main/Input/InputActions/IA_Move.IA_Move"))
  (bind (_x _y) (`KismetMathLibrary.BreakVector2D` ActionValue))
  ;[1 0 1] Controls movement using WASD
  (:`Triggered`
    (set `self.Directionality` ActionValue)
    (`self.AddMovementInput` (1.0 0.0 0.0) _x)
    (`self.AddMovementInput` (0.0 1.0 0.0) _y)
    (`self.f_UpdateAnimation` false))
  (:`Completed`
    (`self.f_UpdateAnimation` true)))

(fn `f_UpdateAnimation`
  (params (`IsTransitionToIdle?` :type Boolean))
  (if `IsTransitionToIdle?`
    (`/Engine/EditorBlueprintResources/StandardMacros.CompareFloat` (`KismetMathLibrary.BreakVector2D` (`self.Directionality`))
      (:`>`
        (`PaperFlipbookComponent.SetFlipbook` (`self.Sprite`) "/Game/_Main/MyAssets/PaperAssets/Characters/Red/FB_Red_Idle_R.FB_Red_Idle_R"))
      (:`==`
        (`/Engine/EditorBlueprintResources/StandardMacros.CompareFloat` (`.Y` (`KismetMathLibrary.BreakVector2D` (`self.Directionality`)))
          (:`>`
            (`PaperFlipbookComponent.SetFlipbook` (`self.Sprite`) "/Game/_Main/MyAssets/PaperAssets/Characters/Red/FB_Red_Idle_D.FB_Red_Idle_D"))
          (:`<`
            (`PaperFlipbookComponent.SetFlipbook` (`self.Sprite`) "/Game/_Main/MyAssets/PaperAssets/Characters/Red/FB_Red_Idle_U.FB_Red_Idle_U"))))
      (:`<`
        (`PaperFlipbookComponent.SetFlipbook` (`self.Sprite`) "/Game/_Main/MyAssets/PaperAssets/Characters/Red/FB_Red_Idle_L.FB_Red_Idle_L")))
    (else
      (`/Engine/EditorBlueprintResources/StandardMacros.CompareFloat` (`KismetMathLibrary.BreakVector2D` (`self.Directionality`))
        (:`>`
          (`PaperFlipbookComponent.SetFlipbook` (`self.Sprite`) "/Game/_Main/MyAssets/PaperAssets/Characters/Red/FB_Red_Walk_R.FB_Red_Walk_R"))
        (:`==`
          (`/Engine/EditorBlueprintResources/StandardMacros.CompareFloat` (`.Y` (`KismetMathLibrary.BreakVector2D` (`self.Directionality`)))
            (:`>`
              (`PaperFlipbookComponent.SetFlipbook` (`self.Sprite`) "/Game/_Main/MyAssets/PaperAssets/Characters/Red/FB_Red_Walk_D.FB_Red_Walk_D"))
            (:`<`
              (`PaperFlipbookComponent.SetFlipbook` (`self.Sprite`) "/Game/_Main/MyAssets/PaperAssets/Characters/Red/FB_Red_Walk_U.FB_Red_Walk_U"))))
        (:`<`
          (`PaperFlipbookComponent.SetFlipbook` (`self.Sprite`) "/Game/_Main/MyAssets/PaperAssets/Characters/Red/FB_Red_Walk_L.FB_Red_Walk_L"))))))

(fn `UserConstructionScript`)